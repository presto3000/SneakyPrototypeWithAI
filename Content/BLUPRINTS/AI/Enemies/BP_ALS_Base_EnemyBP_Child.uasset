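; Base enemy character Blueprint, derived from an ALS-based C++ parent, that sets up an AK47-armed AI with a health bar and alert widget.
; BeginPlay links the health bar to the enemy, spawns the rifle and equips it through the AICombat component.
; Noise-tagged perception stimuli write TargetLocation to the blackboard and briefly show the alert unless stunned.
; Death unpossesses the AI, ragdolls, disables capsule collision, destroys the weapon and sets a lifespan.
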(event `self.ReceiveTick`
  (params (DeltaSeconds :type "Float (single-precision)"))
  (`parent.ReceiveTick` DeltaSeconds))

(event `self.ReceiveBeginPlay`
  (bind _aicombat (`self.AICombat`))
  (bind _startingweapon (`self.StartingWeapon`))
  ;[1 1 1] SetEnemyRef in WB_EnemyHealthBar, Spawn EnemyWeapon, EquipWeapon, HideAlertWidget
  (`parent.ReceiveBeginPlay`)
  (bind _aswb_enemy_health_bar (cast `/Game/BLUPRINTS/UI/WB_EnemyHealthBar` (`WidgetComponent.GetUserWidgetObject` (`self.HealthBarWidget`))))
  (set `/Game/BLUPRINTS/UI/WB_EnemyHealthBar.EnemyRef` self _aswb_enemy_health_bar)
  (`Widget.SetVisibility` _aswb_enemy_health_bar "Hidden")
  (`/Engine/EditorBlueprintResources/StandardMacros.IsValid` _aicombat
    (:`Is Valid`
      (set `AICombatComponent.Character` self _aicombat)
      (bind _returnvalue (`|SpawnActorFromClass` "/Game/BLUPRINTS/Weapons/BP_AK47.BP_AK47_C" (`KismetMathLibrary.MakeTransform` (0.0 0.0 0.0)) "Undefined" "OverrideRootScale" null (`self.GetInstigator`)))
      (set `self.StartingWeapon` _returnvalue)
      (`/Engine/EditorBlueprintResources/StandardMacros.IsValid` _startingweapon
        (:`Is Valid`
          (`AICombatComponent.EquipWeapon` _aicombat _startingweapon)
          (`SceneComponent.SetVisibility` (`self.EnemyAlertNotificationWidget`) false false))))))

(event `self.ShowHealthBar`
  ;[1 1 1] Show HealthBar
  (`Widget.SetVisibility` (`WidgetComponent.GetUserWidgetObject` (`self.HealthBarWidget`)) "Visible")
  ;;[1 1 1] Call cpp
  (`parent.ShowHealthBar`))

(event `self.HideHealthBar`
  ;[1 1 1] Hide HealthBar
  (`Widget.SetVisibility` (`WidgetComponent.GetUserWidgetObject` (`self.HealthBarWidget`)) "Hidden"))

(event `self.AIPerception.OnPerceptionUpdated`
  (params (UpdatedActors :type "Array of Actor Object Reference (by ref)"))
  (bind _returnvalue (`AIBlueprintHelperLibrary.GetBlackboard` null))
  ;[1 1 1] On Perception Updated AI
  (for _array_element UpdatedActors
    (bind _info (`AIPerceptionComponent.GetActorsPerception` (`self.AIPerception`) _array_element))
    (for _array_element_2 (`.LastSensedStimuli` (break `ActorPerceptionBlueprintInfo` _info))
      (bind (_age _expirationage _strength _stimuluslocation _receiverlocation _tag) (break `AIStimulus` _array_element_2))
      (if (== _tag "Noise")
        (`/Engine/EditorBlueprintResources/StandardMacros.IsValid` _returnvalue
          (:`Is Valid`
            (`BlackboardComponent.SetValueAsVector` _returnvalue "TargetLocation" _stimuluslocation)
            (if (`|EnumEquality` (`AICombatComponent.CombatState` (`self.AICombat`)) "Stunned")
              (`SceneComponent.SetVisibility` (`self.EnemyAlertNotificationWidget`) false false)
              (else
                (`SceneComponent.SetVisibility` (`self.EnemyAlertNotificationWidget`) true false)
                (`KismetSystemLibrary.K2_SetTimerDelegate` (delegate `CustomEvent_0`) 3.0)))))))))

(event `CustomEvent_0`
  ;[1 1 1] On Perception Updated AI
  (`SceneComponent.SetVisibility` (`self.EnemyAlertNotificationWidget`) false false))

(event `self.Death`
  (bind _startingweapon (`self.StartingWeapon`))
  (bind _returnvalue (`AIBlueprintHelperLibrary.GetAIController` self))
  (`/Engine/EditorBlueprintResources/StandardMacros.IsValid` _returnvalue
    (:`Is Valid`
      (`Controller.UnPossess` _returnvalue)
      (`self.RagdollStart`)
      (`PrimitiveComponent.SetCollisionEnabled` (`self.CapsuleComponent`) "NoCollision")
      (`self.SetLifeSpan` 4.0)
      (`/Engine/EditorBlueprintResources/StandardMacros.IsValid` _startingweapon
        (:`Is Valid`
          (`self.K2_DestroyActor` _startingweapon))))))

(fn `UserConstructionScript`
  (`parent.UserConstructionScript`))