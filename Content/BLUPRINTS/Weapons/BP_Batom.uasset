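; Baton weapon actor that disables enemies touched by its box collision.
; On both begin and end overlap, it casts the other actor to BP_ALS_Base_EnemyBP_Child and proceeds only if that enemy's starting weapon is valid.
; It then destroys the weapon, starts ragdoll and, if AICombat is valid, sets the combat state to Stunned and unpossesses the enemy's AI controller.
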(event `self.BoxCollisionBatom.OnComponentBeginOverlap`
  (params (OverlappedComponent :type "PrimitiveComponent Object Reference") (OtherActor :type "Actor Object Reference") (OtherComp :type "PrimitiveComponent Object Reference") (OtherBodyIndex :type Integer) (bFromSweep :type Boolean) (SweepResult :type "HitResult Structure (by ref)"))
  (bind _asbp_als_base_enemy_bp_child (cast `/Game/BLUPRINTS/AI/Enemies/BP_ALS_Base_EnemyBP_Child` (stale `self.BoxCollisionBatom.OnComponentEndOverlap` OtherActor) :!label _label))
  (`/Engine/EditorBlueprintResources/StandardMacros.IsValid` _asbp_als_base_enemy_bp_child
    (:`Is Valid`
      (bind _startingweapon (`Enemy.StartingWeapon` _asbp_als_base_enemy_bp_child))
      (`/Engine/EditorBlueprintResources/StandardMacros.IsValid` _startingweapon
        (:`Is Valid`
          (`self.K2_DestroyActor` _startingweapon)
          (`/Game/AdvancedLocomotionV4/Blueprints/CharacterLogic/ALS_Base_EnemyBP.RagdollStart` _asbp_als_base_enemy_bp_child)
          (bind _aicombat (`/Game/BLUPRINTS/AI/Enemies/BP_ALS_Base_EnemyBP_Child.AICombat` _asbp_als_base_enemy_bp_child))
          (`/Engine/EditorBlueprintResources/StandardMacros.IsValid` _aicombat
            (:`Is Valid`
              (set `AICombatComponent.CombatState` "Stunned" _aicombat)
              (bind _returnvalue (`AIBlueprintHelperLibrary.GetAIController` _asbp_als_base_enemy_bp_child))
              (`/Engine/EditorBlueprintResources/StandardMacros.IsValid` _returnvalue
                (:`Is Valid`
                  (`Controller.UnPossess` _returnvalue))))))))))

(event `self.BoxCollisionBatom.OnComponentEndOverlap`
  (params (OverlappedComponent :type "PrimitiveComponent Object Reference") (OtherActor :type "Actor Object Reference") (OtherComp :type "PrimitiveComponent Object Reference") (OtherBodyIndex :type Integer))
  (goto _label))

(fn `UserConstructionScript`)